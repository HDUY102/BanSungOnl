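; BP_ZombiesNor is a zombie enemy that senses the player and feeds that state to its AI Blackboard.
; PawnSensing flags a seen top-down character and, while that player is alive, stores it as the target with an attack flag.
; A sphere overlap sets that attack flag, which reaches the Blackboard only when sight fires.
; Tick refreshes the overhead health bar and hides it at zero health.
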(event OnComponentBeginOverlap(SphereComponent)
  (params (OverlappedComponent :type Primitive%20Component%20Object%20Reference) (OtherActor :type Actor%20Object%20Reference) (OtherComp :type Primitive%20Component%20Object%20Reference) (OtherBodyIndex :type Integer) (bFromSweep :type Boolean) (SweepResult :type Hit%20Result%20Structure%20%28by%20ref%29))
  (Utilities|Casting|CastToBP_TopDownCharacter OtherActor)
  (Variables|Default|SetbAtk true))

(event OnSeePawn(PawnSensing)
  (params (Pawn :type Pawn%20Object%20Reference))
  (bind _returnvalue (Utilities|Name|MakeLiteralName "bATked"))
  (bind _self self)
  (bind _returnvalue_2 (Pawn|GetController _self))
  (bind _returnvalue_3 (AI|GetBlackboard _returnvalue_2))
  ;[0.124 0.124 0.124] Event Behavior Tree
  (bind _asbp_top_down_character (Utilities|Casting|CastToBP_TopDownCharacter Pawn))
  (bind _output_get (Variables|Default|SetPlayerTarget _asbp_top_down_character))
  (AI|Components|Blackboard|SetValueasBool _returnvalue_3 (Utilities|Name|MakeLiteralName "hasSeenPlayer") true)
  (if (not (Variables|/Script/BanSungOnl.BanSungOnlCharacter|GetbIsDead _output_get))
    (AI|Components|Blackboard|SetValueasObject _returnvalue_3 (Variables|Default|GetKey%20Name) _output_get)
    (if (Variables|Default|GetbAtk)
      (AI|Components|Blackboard|SetValueasBool _returnvalue_3 _returnvalue true)
      (else
        (AI|Components|Blackboard|SetValueasBool _returnvalue_3 _returnvalue false)))))

(event OnComponentEndOverlap(SphereComponent)
  (params (OverlappedComponent :type Primitive%20Component%20Object%20Reference) (OtherActor :type Actor%20Object%20Reference) (OtherComp :type Primitive%20Component%20Object%20Reference) (OtherBodyIndex :type Integer))
  (Utilities|Casting|CastToBP_TopDownCharacter OtherActor)
  (Variables|Default|SetbAtk false))

(event Collision|EventActorBeginOverlap
  (params (OtherActor :type Actor%20Object%20Reference)))

(event EventTick
  (params (DeltaSeconds :type Float%20%28single-precision%29))
  (bind _healthzomb (Variables|Default|GetHealthZomb))
  (bind _widgetcomponent (Variables|Default|GetWidgetComponent))
  (if (<= _healthzomb 0.0)
    (Development|SetHiddeninGame _widgetcomponent true false)
    (else
      (bind _aswb_health_ene (Utilities|Casting|CastToWB_HealthEne (UserInterface|GetWidget _widgetcomponent)))
      (Progress|SetPercent (Variables|/Game/UI/WB_HealthEne.WB_HealthEne_C|GetBar_HealthEne _aswb_health_ene) (/ _healthzomb (Variables|Default|GetMaxHealthZomb))))))

(event EventBeginPlay
  (bind _asban_sung_onl_character (Utilities|Casting|CastToBanSungOnlCharacter (Game|GetPlayerCharacter 0)))
  (Variables|Default|SetAs%20Ban%20Sung%20Onl%20Character _asban_sung_onl_character))

(fn ConstructionScript)